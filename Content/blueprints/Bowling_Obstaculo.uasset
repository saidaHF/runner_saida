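; Bowling obstacle that slides along the X axis until a bp_boul actor hits it.
; While IsMovable is set, Tick calls Movement, which overrides the physics velocity of the Bowl component with VelocityX.
; A hit from bp_boul clears IsMovable and adds a force from the hit's normal impulse scaled by VelocityX, also using that impulse vector as the force location.
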(event `self.ReceiveTick`
  (params (DeltaSeconds :type "Float (single-precision)"))
  ;[1 0.7936 0.4853] Call function movement
  (if (`self.isMovable`)
    (`self.Movement` DeltaSeconds)))

(event `self.Bowl.OnComponentHit`
  (params (HitComponent :type "PrimitiveComponent Object Reference") (OtherActor :type "Actor Object Reference") (OtherComp :type "PrimitiveComponent Object Reference") (NormalImpulse :type "Vector Structure") (Hit :type "HitResult Structure (by ref)"))
  ;[0.1765 1 0.9702] Event collide
  (cast `/Game/blueprints/bp_boul` OtherActor)
  (set `self.isMovable` false) ; Check = true, not check = false
  (`PrimitiveComponent.AddForceAtLocation` (`self.Bowl`) (* NormalImpulse (* (`self.velocity X`) 10.0)) NormalImpulse "None"))

(fn `Movement`
  (params (DataTime :type "Float (double-precision)"))
  (`PrimitiveComponent.SetPhysicsLinearVelocity` (`self.Bowl`) (`KismetMathLibrary.MakeVector` (`self.velocity X`)) false "None"))

(fn `UserConstructionScript`)