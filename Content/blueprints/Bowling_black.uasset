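; Bowling_black is a bowling Blueprint that reacts to being struck by a bp_boul object and then ends the game.
; Its Collision function, when passed a bp_boul while IsMovable is set, clears that flag and applies a force to Bowl at the given location, scaled by VelocityX.
; It then immediately calls QuitGame.
; The event graph holds only disabled default events.
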(fn `Collision`
  (params (Location :type "Vector Structure") (A :type "Vector Structure") (Object :type "Object Object Reference"))
  ;[0.1765 1 0.9702] Event collide
  (cast `/Game/blueprints/bp_boul` Object)
  (if (`self.isMovable`)
    (set `self.isMovable` false) ; Check = true, not check = false
    (`PrimitiveComponent.AddForceAtLocation` (`self.Bowl`) (* A (* (`self.velocity X`) 10.0)) Location "None")
    (`KismetSystemLibrary.QuitGame` null "Quit")))

(fn `UserConstructionScript`
  (`parent.UserConstructionScript`))