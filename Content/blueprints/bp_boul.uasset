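; Player-controlled physics ball (boule) that moves left and right along the Y axis with the A and D keys.
; The Movement axis event damps the sphere's lateral velocity by a fixed factor, zeroes X and keeps Z, then applies a mass-independent force scaled by input and Velocity.
; The construction script only prints a debug string, and the Move function is an empty stub.
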(event `InputAxis|Movement`
  (params (AxisValue :type "Float (single-precision)"))
  (bind _sphere_boul (`self.sphere_boul`))
  ;[0.8636 0.5873 1] Movement L-R (key A and key D)
  (bind _returnvalue (`PrimitiveComponent.GetPhysicsLinearVelocity` _sphere_boul "None"))
  (`PrimitiveComponent.SetPhysicsLinearVelocity` _sphere_boul (`KismetMathLibrary.MakeVector` 0.0 (* (.y _returnvalue) 0.9) (.z _returnvalue)) false "None")
  (`PrimitiveComponent.AddForce` (`self.sphere_boul`) (`KismetMathLibrary.MakeVector` 0.0 (* (* AxisValue (`.Y` (`KismetMathLibrary.BreakVector3f` (0.0 1.0 0.0)))) (`self.velocity`))) "None" true))

(fn `Move`)

(fn `UserConstructionScript`
  (`KismetSystemLibrary.PrintString` "Hello"))