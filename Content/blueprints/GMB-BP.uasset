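; GMB-BP is a game mode Blueprint that keeps the score and shows it on screen.
; On BeginPlay it creates the PointInterface widget for the first player controller and adds it to the viewport, unless one already exists.
; AddPoints adds the given amount to the Points total and, when the widget is valid, passes the new total to its SetTextScore.
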(event `self.ReceiveBeginPlay`
  (`/Engine/EditorBlueprintResources/StandardMacros.IsValid` (`self.PointInterface`)
    (:`Is Not Valid`
      (bind _returnvalue (`|CreateWidget` "/Game/blueprints/pointInterface.pointInterface_C" (`GameplayStatics.GetPlayerController` 0)))
      (bind _output_get (set `self.PointInterface` _returnvalue))
      (`UserWidget.AddToViewport` _output_get 0))))

(fn `AddPoints`
  (params (newPoint :type Integer))
  (bind _pointinterface (`self.PointInterface`))
  ;[0.4616 1 0.296] Function add points in the text
  (set `self.Points` (+ newPoint (`self.Points`)))
  (`/Engine/EditorBlueprintResources/StandardMacros.IsValid` _pointinterface
    (:`Is Valid`
      (`/Game/blueprints/pointInterface.setTextScore` _pointinterface (`self.Points`)))))

(fn `UserConstructionScript`)