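; Bowling obstacle that moves under physics and awards points to the game mode when a bp_boul hits it.
; While IsMovable, Tick drives the Bowl component's linear velocity from VelocityX.
; The first qualifying hit clears IsMovable, applies a force scaled from the normal impulse and VelocityX, and adds NewPoint through the GMB-BP cached at BeginPlay.
; The normal impulse also serves as the force's location.
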(event `self.ReceiveBeginPlay`
  ;[0.9247 0.1517 1] Save the GMB-BP
  (bind _asgmb_bp (cast `/Game/blueprints/GMB-BP` (`GameplayStatics.GetGameMode`)))
  (set `self.gamemode_GMB-BP` _asgmb_bp))

(event `self.ReceiveTick`
  (params (DeltaSeconds :type "Float (single-precision)"))
  ;[1 0.7936 0.4853] Call function movement
  (if (`self.isMovable`)
    (`self.Movement` DeltaSeconds)))

(event `self.Bowl.OnComponentHit`
  (params (HitComponent :type "PrimitiveComponent Object Reference") (OtherActor :type "Actor Object Reference") (OtherComp :type "PrimitiveComponent Object Reference") (NormalImpulse :type "Vector Structure") (Hit :type "HitResult Structure (by ref)"))
  ;[1 1 1] Collision
  (`self.Collision` NormalImpulse NormalImpulse OtherActor))

(fn `Collision`
  (params (Location :type "Vector Structure") (A :type "Vector Structure") (Object :type "Object Object Reference"))
  ;[0.1765 1 0.9702] Event collide
  (cast `/Game/blueprints/bp_boul` Object)
  (if (`self.isMovable`)
    (set `self.isMovable` false) ; Check = true, not check = false
    (`PrimitiveComponent.AddForceAtLocation` (`self.Bowl`) (* A (* (`self.velocity X`) 10.0)) Location "None")
    (`/Game/blueprints/GMB-BP.AddPoints` (`self.gamemode_GMB-BP`) (`self.New Point`))))

(fn `Movement`
  (params (DataTime :type "Float (double-precision)"))
  (`PrimitiveComponent.SetPhysicsLinearVelocity` (`self.Bowl`) (`KismetMathLibrary.MakeVector` (`self.velocity X`)) false "None"))

(fn `UserConstructionScript`)